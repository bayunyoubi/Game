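; Boss actor that watches the player and adjusts affection values stored in the Varibles game instance.
; Tick line-traces forward from a StaticMesh and accumulates how long the first-person character stays in sight.
; Brief sightings penalize PlayerLove for phone use; longer ones clear the phone flag, then raise BossLove if Stand is set, otherwise lower PlayerLove, via delayed timers.
; LookAt, uncalled here, plays head-turn animations within fixed game-time windows.
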(event Custom|SubstractLove
  ;[1 1 1] 扣好感度
  (bind _asvaribles (Utilities|Casting|CastToVaribles (Game|GetGameInstance)))
  (Variables|/Game/BluePrints/Varibles.Varibles_C|SetPlayLove _asvaribles (Utilities|Struct|MakePlayer (- (.playerlove (Variables|/Game/BluePrints/Varibles.Varibles_C|GetPlayLove _asvaribles)) 1) (.islookingphone (Variables|/Game/BluePrints/Varibles.Varibles_C|GetPlayLove _asvaribles)) (.stand (Variables|/Game/BluePrints/Varibles.Varibles_C|GetPlayLove _asvaribles)))))

(event Custom|LookStand
  (bind _asvaribles (Utilities|Casting|CastToVaribles (Game|GetGameInstance)))
  (Variables|/Game/BluePrints/Varibles.Varibles_C|SetPlayLove _asvaribles (Utilities|Struct|MakePlayer (.playerlove (Variables|/Game/BluePrints/Varibles.Varibles_C|GetPlayLove _asvaribles)) false (.stand (Variables|/Game/BluePrints/Varibles.Varibles_C|GetPlayLove _asvaribles))))
  (if (.stand (Variables|/Game/BluePrints/Varibles.Varibles_C|GetPlayLove _asvaribles))
    (Utilities|FlowControl|Delay 2.0)
    (Utilities|Time|SetTimerbyFunctionName 0 "Addlove" 1.0)
    (else
      (Utilities|FlowControl|Delay 2.0)
      (Utilities|Time|SetTimerbyEvent (delegate Custom|Delete%20Love) 1.0))))

(event Custom|LookAt
  ;[1 1 1] 固定时间转头
  (Utilities|FlowControl|Sequence
    (:then_0
      (if (Math|Float|InRange(Float) (Utilities|Time|GetGameTimeinSeconds) 5.0 1e+01)
        (Components|Animation|PlayAnimation (Variables|Character|GetMesh) "/Game/Animation/LookAroundLeft45.LookAroundLeft45" true)
        (Utilities|FlowControl|Delay 5.0)
        (Components|Animation|PlayAnimation (Variables|Character|GetMesh) "/Game/Animation/Sitting_Idle.Sitting_Idle" true)))
    (:then_1
      (if (Math|Float|InRange(Float) (Utilities|Time|GetGameTimeinSeconds) 2e+01 35.0)
        (Components|Animation|PlayAnimation (Variables|Character|GetMesh) "/Game/Animation/LookAroundLeft45.LookAroundLeft45" true)
        (Utilities|FlowControl|Delay 5.0)
        (Components|Animation|PlayAnimation (Variables|Character|GetMesh) "/Game/Animation/Sitting_Idle.Sitting_Idle" true)))
    (:then_2
      (if (Math|Float|InRange(Float) (Utilities|Time|GetGameTimeinSeconds) 55.0 6e+01)
        (Components|Animation|PlayAnimation (Variables|Character|GetMesh) "/Game/Animation/LookAroundLeft45.LookAroundLeft45" true)
        (Utilities|FlowControl|Delay 5.0)
        (Components|Animation|PlayAnimation (Variables|Character|GetMesh) "/Game/Animation/Sitting_Idle.Sitting_Idle" true)))))

(event Custom|LookPhone
  ;[1 1 1] 注释
  (bind _asvaribles (Utilities|Casting|CastToVaribles (Game|GetGameInstance)))
  (if (.islookingphone (Variables|/Game/BluePrints/Varibles.Varibles_C|GetPlayLove _asvaribles))
    (Utilities|FlowControl|Delay 1.5)
    (Utilities|Time|SetTimerbyEvent (delegate Custom|SubstractLove) 1.0)))

(event Custom|Delete%20Love
  (bind _asvaribles (Utilities|Casting|CastToVaribles (Game|GetGameInstance)))
  (bind _output_get (Variables|/Game/BluePrints/Varibles.Varibles_C|SetPlayLove _asvaribles (Utilities|Struct|MakePlayer (- (.playerlove (Variables|/Game/BluePrints/Varibles.Varibles_C|GetPlayLove _asvaribles)) 2) (.islookingphone (Variables|/Game/BluePrints/Varibles.Varibles_C|GetPlayLove _asvaribles)) (.stand (Variables|/Game/BluePrints/Varibles.Varibles_C|GetPlayLove _asvaribles)))))
  (Development|PrintString (Utilities|String|ToString(Integer) (.playerlove _output_get))))

(event EventBeginPlay)

(event Collision|EventActorBeginOverlap
  (params (OtherActor :type Actor%20Object%20Reference)))

(event EventTick
  (params (DeltaSeconds :type Float%20%28single-precision%29))
  (bind _staticmesh (Variables|Default|GetStaticMesh))
  (bind _returnvalue (Transformation|GetWorldLocation _staticmesh))
  ;[1 1 1] 视线检测
  (bind _outhit (Collision|LineTraceForObjects _returnvalue (+ _returnvalue (* (Math|Vector|GetForwardVector _staticmesh) (Variables|Default|GetDisdance)) "") (Utilities|Array|MakeArray "ObjectTypeQuery3") false 0 "None" true "(R=1.000000,G=0.000000,B=0.000000,A=1.000000)" "(R=0.000000,G=1.000000,B=0.000000,A=1.000000)" 0.1))
  (if (Utilities|Enum|Equal(Enum) (Utilities|GetDisplayName (.HitActor (Collision|BreakHitResult _outhit))) "BP_FirstPersonCharacter")
    (Variables|Default|SetLookTime (+ (Variables|Default|GetLookTime) DeltaSeconds))
    (if (>= (Variables|Default|GetLookTime) 3.0)
      (CallFunction|LookStand)
      (else
        (CallFunction|LookPhone)))
    (else
      (Variables|Default|SetLookTime 0.0))))

(fn ConstructionScript)

(fn Addlove
  (bind _asvaribles (Utilities|Casting|CastToVaribles (Game|GetGameInstance)))
  (bind _output_get (Variables|/Game/BluePrints/Varibles.Varibles_C|SetBossLove _asvaribles (Utilities|Struct|MakeBossBase (+ (.bosslove (Variables|/Game/BluePrints/Varibles.Varibles_C|GetBossLove _asvaribles)) 2) (.issee (Variables|/Game/BluePrints/Varibles.Varibles_C|GetBossLove _asvaribles)) (.1 (Variables|/Game/BluePrints/Varibles.Varibles_C|GetBossLove _asvaribles)) (.2 (Variables|/Game/BluePrints/Varibles.Varibles_C|GetBossLove _asvaribles)) (.3 (Variables|/Game/BluePrints/Varibles.Varibles_C|GetBossLove _asvaribles)))))
  (Development|PrintString (Utilities|String|ToString(Integer) (.bosslove _output_get))))