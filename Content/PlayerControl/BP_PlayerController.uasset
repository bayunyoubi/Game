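; Player controller Blueprint that owns the player's UI: the main HUD and the pause menu.
; On BeginPlay it creates MainHUD and shows the mouse cursor; Escape spawns a new PauseMenu widget on each press.
; Custom events forward mood updates for player and boss, and render requests, to the HUD's ScaleWidget.
; The 2 key prints the player's current mood value from that widget.
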(event Custom|RenderingScale
  (Default|RenderingScale (Variables|/Game/UI/MainHUD.MainHUD_C|GetScaleWidget (stale EventBeginPlay _returnvalue))))

(event Custom|Custom%20Change%20Mood%20and%20Rendering
  (params (NewPlayerMoodValue :type Float%20%28double-precision%29) (NewBossMoodValue :type Float%20%28double-precision%29))
  (Default|ChangeMoodandRendering (Variables|/Game/UI/MainHUD.MainHUD_C|GetScaleWidget (stale EventBeginPlay _returnvalue)) NewPlayerMoodValue NewBossMoodValue))

(event EventBeginPlay
  (bind _returnvalue (UserInterface|CreateWidget "/Game/UI/MainHUD.MainHUD_C"))
  (UserInterface|Viewport|AddtoViewport _returnvalue 0)
  (Variables|/Script/Engine.PlayerController|SetbShowMouseCursor (Game|GetPlayerController 0) true))

(event EventTick
  (params (DeltaSeconds :type Float%20%28single-precision%29)))

(event Input|KeyboardEvents|Escape
  (params (Key :type Key%20Structure :default "None"))
  ;[1 1 1] PauseMenuPopUp
  (:Pressed
    (bind _returnvalue (UserInterface|CreateWidget "/Game/UI/PauseMenu.PauseMenu_C"))
    (UserInterface|Viewport|AddtoViewport _returnvalue 0)
    (Variables|/Script/Engine.PlayerController|SetbShowMouseCursor (Game|GetPlayerController 0) true)))

(event Input|KeyboardEvents|2
  (params (Key :type Key%20Structure :default "None"))
  (:Pressed
    (Development|PrintString (Utilities|String|ToString(Float) (Variables|/Game/UI/ScaleWidget.ScaleWidget_C|GetPlayerMoodValue (Variables|/Game/UI/MainHUD.MainHUD_C|GetScaleWidget (stale EventBeginPlay _returnvalue)))))))

(fn ConstructionScript)